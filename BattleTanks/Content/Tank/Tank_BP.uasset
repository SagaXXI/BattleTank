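; Tank_BP is the tank pawn that turns player input into driving, aiming, firing and camera switching.
; Input axes drive the TankMovement component and rotate an azimuth gimbal and spring arm for looking around, while actions fire via TankAiming or toggle first and third person cameras.
; BeginPlay wires barrel, turret and tracks into those components, adds a HUD only when player controlled, and hands itself to its health bar widget.
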(event Collision|EventActorBeginOverlap
  (params (OtherActor :type Actor%20Object%20Reference)))

(event EventTick
  (params (DeltaSeconds :type Float%20%28single-precision%29)))

(event EventBeginPlay
  ;[1 1 1] Setup
  (if (Pawn|IsPlayerControlled)
    (CallFunction|SetupUI))
  (Class|TankAimingComponent|Initialise (Variables|Default|GetTankAiming) (Variables|Default|GetTankBarrel) (Variables|Default|GetTankTurret))
  (Class|TankMovementComponent|Initialise (Variables|Default|GetTankMovement) (Variables|Default|GetLeftTrack) (Variables|Default|GetRightTrack))
  (CallFunction|SetHealthBar))

(event Input|ActionEvents|InputActionFire
  (params (Key :type Key%20Structure))
  ;[1 1 1] Bind the fire function here ok?
  (:Pressed
    (Class|TankAimingComponent|Fire (Variables|Default|GetTankAiming))))

(event Input|ActionEvents|InputActionViewchanging
  (params (Key :type Key%20Structure))
  ;[1 1 1] Camera Input Binding
  (:Pressed
    (Components|Activation|ToggleActive (Variables|Default|Get1st%20person))
    (Components|Activation|ToggleActive (Variables|Default|Get3rd%20person))))

(event Input|AxisEvents|InputAxisAimAzimuth
  (params (AxisValue :type Float%20%28single-precision%29))
  ;[1 1 1] Camera Input Binding
  (Transformation|AddLocalRotation (Variables|Default|GetAzimuth%20Gimbal) (Math|Rotator|MakeRotator 0.0 0.0 AxisValue) false false))

(event Input|AxisEvents|InputAxisAimElevation
  (params (AxisValue :type Float%20%28single-precision%29))
  ;[1 1 1] Camera Input Binding
  (Transformation|AddLocalRotation (Variables|Default|GetSpringArm) (Math|Rotator|MakeRotator 0.0 AxisValue 0.0) false false))

(event Input|AxisEvents|InputAxisMoveForward
  (params (AxisValue :type Float%20%28single-precision%29))
  ;[1 1 1] Movement binding
  (Class|TankMovementComponent|IntendMoveForward (Variables|Default|GetTankMovement) AxisValue))

(event Input|AxisEvents|InputAxisTurnRight
  (params (AxisValue :type Float%20%28single-precision%29))
  ;[1 1 1] Movement binding
  (Class|TankMovementComponent|IntendTurnRight (Variables|Default|GetTankMovement) AxisValue))

(fn ConstructionScript)

(fn SetupUI
  (bind _returnvalue (UserInterface|CreateWidget "/Game/UI/WBP_PlayerUI.WBP_PlayerUI_C"))
  (Variables|/Game/UI/WBP_PlayerUI.WBP_PlayerUI_C|SetTank%20Aim%20Comp%20Ref _returnvalue (Variables|Default|GetTankAiming))
  (UserInterface|Viewport|AddtoViewport _returnvalue 0))

(fn SetHealthBar
  (bind _aswbp_health_bar (Utilities|Casting|CastToWBP_HealthBar (UserInterface|GetUserWidgetObject (Variables|Default|GetWidget))))
  (Variables|/Game/UI/WBP_HealthBar.WBP_HealthBar_C|SetTankRef _aswbp_health_bar self))